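; Tile spawner actor that builds and extends a chain of BP__TILE actors, as for an endless track.
; On BeginPlay it spawns an initial run of tiles, the first at the world origin and each next one at the SpawnPoint of the newest tile.
; Each spawned tile becomes NewestTile and receives a reference back to the spawner, with SpawnTileAtSpawnPoint available to append another tile.
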(event `self.ReceiveBeginPlay`
  (`self.SpawnInitialTiles`))

(fn `SpawnInitialTiles`
  (for _ (range 6)
    (`/Engine/EditorBlueprintResources/StandardMacros.IsValid` (`self.Newest Tile`)
      (:`Is Valid`
        (`self.SpawnTileAtSpawnPoint`))
      (:`Is Not Valid`
        (`self.SpawnTile` (0.0 0.0 0.0))))))

(fn `SpawnTile`
  (params (Spawnlocation :type "Vector Structure"))
  (locals (NewLocalVar_0 :type "Transform Structure"))
  (bind _returnvalue (`|SpawnActorFromClass` "/Game/BP__TILE.BP__TILE_C" (`KismetMathLibrary.MakeTransform` Spawnlocation) "Undefined" "OverrideRootScale" null null))
  (bind _output_get (set `self.Newest Tile` _returnvalue))
  (set `/Game/BP__TILE.TileSpawner` self _output_get))

(fn `SpawnTileAtSpawnPoint`
  (`self.SpawnTile` (`SceneComponent.K2_GetComponentLocation` (`/Game/BP__TILE.SpawnPoint` (`self.Newest Tile`)))))

(fn `UserConstructionScript`)