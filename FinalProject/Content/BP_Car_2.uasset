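; BP_Car_2 is a car actor that shuttles back and forth between its StartPoint and EndPoint.
; BeginPlay caches both points' world locations, picks a random speed and sets the first target from MoveToStart.
; Tick moves the actor at constant speed with VInterpToConstant, without sweep or rotation change.
; On reaching the target, it flips MoveToStart and heads for the other point.
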(event `self.ReceiveBeginPlay`
  (set `self.Current Location` (`self.K2_GetActorLocation`))
  (set `self.Start Point location` (`SceneComponent.K2_GetComponentLocation` (`self.Start Point`)))
  (set `self.End Point location` (`SceneComponent.K2_GetComponentLocation` (`self.End Point`)))
  (set `self.Movment Speed` (`KismetMathLibrary.RandomFloatInRange` 5000.0 10000.0))
  (if (`self.Move To Start`)
    (set `self.Target Location` (`self.Start Point location`))
    (else
      (set `self.Target Location` (`self.End Point location`)))))

(event `self.ReceiveTick`
  (params (DeltaSeconds :type "Float (single-precision)"))
  (set `self.Frame Time` DeltaSeconds)
  (bind _output_get (set `self.Current Location` (`KismetMathLibrary.VInterpTo_Constant` (`self.Current Location`) (`self.Target Location`) (`self.Frame Time`) (`self.Movment Speed`))))
  (`self.K2_SetActorLocation` _output_get)
  (if (<= (`KismetMathLibrary.VSize` (- (`self.K2_GetActorLocation`) (`self.Target Location`))) 0.0)
    (if (`self.Move To Start`)
      (set `self.Target Location` (`self.End Point location`))
      (set `self.Move To Start` false)
      (else
        (set `self.Target Location` (`self.Start Point location`))
        (set `self.Move To Start` true)))))

(fn `UserConstructionScript`)