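; Player actor that is pushed along X by physics impulses, scores by distance and ends the run on a hit.
; Overlaps on four Body components set a Hit flag.
; The Forward axis event applies mass- and frame-time-scaled impulses using delta seconds cached on Tick, and derives Score from X position.
; The same event checks Hit, then plays an explosion, destroys the actor and shows the End widget and mouse cursor.
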(event `self.Body3.OnComponentBeginOverlap`
  (params (OverlappedComponent :type "PrimitiveComponent Object Reference") (OtherActor :type "Actor Object Reference") (OtherComp :type "PrimitiveComponent Object Reference") (OtherBodyIndex :type Integer) (bFromSweep :type Boolean) (SweepResult :type "HitResult Structure (by ref)"))
  (set `self.Hit` true))

(event `self.Body2.OnComponentBeginOverlap`
  (params (OverlappedComponent :type "PrimitiveComponent Object Reference") (OtherActor :type "Actor Object Reference") (OtherComp :type "PrimitiveComponent Object Reference") (OtherBodyIndex :type Integer) (bFromSweep :type Boolean) (SweepResult :type "HitResult Structure (by ref)"))
  (set `self.Hit` true))

(event `self.Body.OnComponentBeginOverlap`
  (params (OverlappedComponent :type "PrimitiveComponent Object Reference") (OtherActor :type "Actor Object Reference") (OtherComp :type "PrimitiveComponent Object Reference") (OtherBodyIndex :type Integer) (bFromSweep :type Boolean) (SweepResult :type "HitResult Structure (by ref)"))
  (set `self.Hit` true))

(event `self.Body1.OnComponentBeginOverlap`
  (params (OverlappedComponent :type "PrimitiveComponent Object Reference") (OtherActor :type "Actor Object Reference") (OtherComp :type "PrimitiveComponent Object Reference") (OtherBodyIndex :type Integer) (bFromSweep :type Boolean) (SweepResult :type "HitResult Structure (by ref)"))
  (set `self.Hit` true))

(event `InputAxis|Forward`
  (params (AxisValue :type "Float (single-precision)"))
  (`PrimitiveComponent.AddImpulse` (`self.Player`) (`KismetMathLibrary.MakeVector` (* AxisValue (* (stale `self.ReceiveTick` _output_get) (* (`PrimitiveComponent.GetMass` (`self.Player`)) (`self.Forward Force`))))) "None" false)
  (set `self.Score` (/ (`KismetMathLibrary.Round` (.x (`SceneComponent.K2_GetComponentLocation` (`self.Player`)))) 100))
  (if (`self.Hit`)
    (`GameplayStatics.PlaySound2D` "/Game/StarterContent/Audio/Explosion02.Explosion02" 1.0 1.0 0.0 null null)
    (`self.K2_DestroyActor`)
    (bind _returnvalue (`|CreateWidget` "/Game/End.End_C"))
    (`UserWidget.AddToViewport` _returnvalue 0)
    (set `PlayerController.bShowMouseCursor` true (`GameplayStatics.GetPlayerController` 0))))

(event `self.ReceiveTick`
  (params (DeltaSeconds :type "Float (single-precision)"))
  (bind _output_get (set `self.Delta Seconds` DeltaSeconds)))

(fn `UserConstructionScript`)